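; BlinkingLight is a Blueprint that drives its BLight component as a switchable light with an optional random flicker.
; Tick reads LightOn and Blinking to set the intensity to zero, steady full brightness or a random level up to full.
; A short Delay inside Tick throttles the flicker, so the intensity changes at intervals instead of every frame.
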(event `self.ReceiveBeginPlay`)

(event `self.ReceiveTick`
  (params (DeltaSeconds :type "Float (single-precision)"))
  (bind _blight (`self.bLight`))
  (if (`self.LightOn`)
    (if (`self.Blinking`)
      (`KismetSystemLibrary.Delay` 0.05)
      (`LightComponent.SetIntensity` (`self.bLight`) (`KismetMathLibrary.RandomFloatInRange` 0.0 3500.0))
      (else
        (`LightComponent.SetIntensity` _blight 3500.0)))
    (else
      (`LightComponent.SetIntensity` _blight 0.0))))

(fn `UserConstructionScript`)